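; BP_ToggleDoor is a door actor that opens by moving straight up and closes by returning to its starting height.
; BeginPlay records the closed Z from its placement and an open Z a fixed offset above it.
; OpenDoor and CloseDoor events snap the actor between those heights with no interpolation or sweep.
; The construction script adds a cube mesh scaled into a thin, tall panel.
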(event `self.ReceiveBeginPlay`
  (bind _returnvalue (`self.K2_GetActorLocation`))
  (set `self.ClosedZ` (.z _returnvalue))
  (set `self.OpenZ` (+ (.z _returnvalue) 300.0)))

(event `OpenDoor`
  (bind _returnvalue (`self.K2_GetActorLocation`))
  (`self.K2_SetActorLocation` (`KismetMathLibrary.MakeVector` (.x _returnvalue) (.y _returnvalue) (`self.OpenZ`))))

(event `CloseDoor`
  (bind _returnvalue (`self.K2_GetActorLocation`))
  (`self.K2_SetActorLocation` (`KismetMathLibrary.MakeVector` (.x _returnvalue) (.y _returnvalue) (`self.ClosedZ`))))

(fn `UserConstructionScript`
  (bind _returnvalue (`AddComponent|NODE_AddStaticMeshComponent-1`))
  (`StaticMeshComponent.SetStaticMesh` _returnvalue "/Engine/BasicShapes/Cube.Cube")
  (`SceneComponent.SetRelativeScale3D` _returnvalue (`KismetMathLibrary.MakeVector` 0.2 2.0 3.0)))