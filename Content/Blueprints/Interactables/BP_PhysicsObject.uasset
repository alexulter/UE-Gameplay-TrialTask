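; Physics object actor that returns to its starting transform when it falls below a height threshold.
; BeginPlay caches the StaticMesh world location and rotation, and Tick compares the mesh's Z against FallRespawnZThreshold.
; On respawn, RespawnAtStart teleports both the simulated mesh and the actor back, zeroing linear and angular velocity before and after the move so no momentum carries over.
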(event `self.ReceiveBeginPlay`
  (bind _staticmesh (`self.StaticMesh`))
  (set `self.InitialLocation` (`SceneComponent.K2_GetComponentLocation` _staticmesh))
  (set `self.InitialRotation` (`SceneComponent.K2_GetComponentRotation` _staticmesh)))

(event `self.ReceiveTick`
  (params (DeltaSeconds :type "Float (single-precision)"))
  (`self.CheckFallAndRespawn`))

(fn `CheckFallAndRespawn`
  (if (< (.z (`SceneComponent.K2_GetComponentLocation` (`self.StaticMesh`))) (`self.FallRespawnZThreshold`))
    (`self.RespawnAtStart`)))

(fn `RespawnAtStart`
  (bind _returnvalue (`KismetMathLibrary.MakeVector` 0.0))
  (bind _staticmesh (`self.StaticMesh`))
  (bind _initiallocation (`self.InitialLocation`))
  (bind _initialrotation (`self.InitialRotation`))
  (`PrimitiveComponent.SetPhysicsLinearVelocity` _staticmesh _returnvalue false "None")
  (`PrimitiveComponent.SetPhysicsAngularVelocityInDegrees` _staticmesh _returnvalue false "None")
  (`SceneComponent.K2_SetWorldLocationAndRotation` _staticmesh _initiallocation _initialrotation false true)
  (`self.K2_TeleportTo` self _initiallocation _initialrotation)
  (`PrimitiveComponent.SetPhysicsLinearVelocity` _staticmesh _returnvalue false "None")
  (`PrimitiveComponent.SetPhysicsAngularVelocityInDegrees` _staticmesh _returnvalue false "None"))

(fn `UserConstructionScript`)